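; BP_SoundTrigger is a one-shot trigger volume that plays a 2D sound when the player character enters its box.
; Before playback it sends a Turn message with one signal to the TurnBeforePlay items.
; After a delay equal to the sound's duration, it sends the TurnAfterPlay items the other signal.
; TurnItems loops over each list and calls TurnMessage on every element.
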(event `self.Box.OnComponentBeginOverlap`
  (params (OverlappedComponent :type "PrimitiveComponent Object Reference") (OtherActor :type "Actor Object Reference") (OtherComp :type "PrimitiveComponent Object Reference") (OtherBodyIndex :type Integer) (bFromSweep :type Boolean) (SweepResult :type "HitResult Structure (by ref)"))
  (bind _sound (`self.sound`))
  (if (== OtherActor (`GameplayStatics.GetPlayerCharacter` 0))
    (`/Engine/EditorBlueprintResources/StandardMacros.DoOnce` false
      (:`Completed`
        (`self.Turn Items` (`self.Turn Before Play`) "NewEnumerator1")
        (`GameplayStatics.PlaySound2D` _sound 1.0 1.0 0.0 null null)
        (`KismetSystemLibrary.Delay` (`SoundBase.Duration` _sound))
        (`self.Turn Items` (`self.Turn After Play`))))))

(fn `Turn Items`
  (params (items :type "Array of Actor Object Reference") (signal :type "/Game/Assets/FPSPuzzleSP/Blueprints/Components/Enum_Signal Enum" :default "NewEnumerator0"))
  (if (> (`KismetArrayLibrary.Array_Length` items) 0)
    (for _array_element items
      (message `/Game/Assets/FPSPuzzleSP/Blueprints/Components/BI_Signal.Turn` _array_element signal))))

(fn `UserConstructionScript`)