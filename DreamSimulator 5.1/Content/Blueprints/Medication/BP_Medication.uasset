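; BP_Medication is a medication pickup that raises the MedicinesLeft count in BP_GameInstance when collected.
; Each Tick, if ActorIsNear passes, left mouse is held and the Avaliable flag is set, it runs an FL_PuzzleLib trace ignoring the player pawn.
; A hit on any BP_Medication, not specifically itself, clears the flag, increments the count, destroys this actor and plays an equip sound.
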(event `self.ReceiveTick`
  (params (DeltaSeconds :type "Float (single-precision)"))
  (bind _is_near (`/Game/Assets/FPSPuzzleSP/Blueprints/Components/FL_PuzzleLib.ActorIsNear` self))
  (if (and _is_near (`PlayerController.IsInputKeyDown` (`GameplayStatics.GetPlayerController` 0) "LeftMouseButton") (`self.Avaliable`))
    (bind (_outhit _returnvalue _hitactor) (`/Game/Assets/FPSPuzzleSP/Blueprints/Components/FL_PuzzleLib.TraceFromActor` 400.0 "TraceTypeQuery1" false (`|MakeArray` (`GameplayStatics.GetPlayerPawn` 0) :!type "Actor Object Reference"))) ; FL_PuzzleLib
    (cast `/Game/Blueprints/Medication/BP_Medication` _hitactor)
    (set `self.Avaliable` false)
    (bind _asbp_game_instance (cast `/Game/BP_GameInstance` (`GameplayStatics.GetGameInstance`)))
    (`/Engine/EditorBlueprintResources/StandardMacros.IncrementInt` (`/Game/BP_GameInstance.Medicines Left` _asbp_game_instance)
      (:`  `
        (`self.K2_DestroyActor`)
        (`GameplayStatics.PlaySound2D` "/Game/Assets/Sounds/ItemEquip.ItemEquip" 1.0 1.0 0.0 null null)
        (`KismetSystemLibrary.Delay` 0.2)
        (set `self.Avaliable` true)))))

(fn `UserConstructionScript`)